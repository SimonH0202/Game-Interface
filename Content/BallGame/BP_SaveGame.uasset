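; BP_SaveGame stores and restores the ball game's cube settings: minimum and maximum size and speed.
; SaveGame creates a save object, copies the current cube values into it and writes it to a fixed "savegame" slot.
; LoadGame reads that slot and returns the values as outputs, stopping at the cast if no valid save object is found.
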(fn SaveGame
  (bind _returnvalue (SaveGame|CreateSaveGameObject))
  (bind _asbp_save_game (Utilities|Casting|CastToBP_SaveGame _returnvalue))
  (Variables|BP_SaveGame_C|SetCubeSizeMin _asbp_save_game (Variables|Default|GetCubeSizeMin))
  (Variables|BP_SaveGame_C|SetCubeSizeMax _asbp_save_game (Variables|Default|GetCubeSizeMax))
  (Variables|BP_SaveGame_C|SetCubeSpeedMin _asbp_save_game (Variables|Default|GetCubeSpeedMin))
  (Variables|BP_SaveGame_C|SetCubeSpeedMax _asbp_save_game (Variables|Default|GetCubeSpeedMax))
  (SaveGame|SaveGametoSlot _asbp_save_game "savegame"))

(fn LoadGame
  (bind _returnvalue (SaveGame|LoadGamefromSlot "savegame"))
  (bind _asbp_save_game (Utilities|Casting|CastToBP_SaveGame _returnvalue))
  (return (Variables|BP_SaveGame_C|GetCubeSizeMin _asbp_save_game) (Variables|BP_SaveGame_C|GetCubeSizeMax _asbp_save_game) (Variables|BP_SaveGame_C|GetCubeSpeedMin _asbp_save_game) (Variables|BP_SaveGame_C|GetCubeSpeedMax _asbp_save_game)))