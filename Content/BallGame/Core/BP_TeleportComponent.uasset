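; Scene component that teleports its owning actor to a spot aimed along the component's forward vector.
; On BeginPlay it spawns a BP_TeleportTarget marker and caches the owner's capsule half-height as a Z offset.
; While teleporting is active, Tick line-traces forward and moves the marker to the hit point projected onto navigation.
; StopTeleport hides the marker and, if the trace hit, moves the owner there, raised by that offset.
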(event EventBeginPlay
  (bind _output_get (Variables|Default|SetTeleportActor (Components|GetOwner)))
  (CallFunction|GetZOffset _output_get)
  (bind _returnvalue (Game|SpawnActorfromClass "/Game/BallGame/BP_TeleportTarget.BP_TeleportTarget_C" (Math|Transform|MakeTransform "0, 0, 0") "Undefined" 0 0))
  (Variables|Default|SetTeleportTarget _returnvalue))

(event EventTick
  (params (DeltaSeconds :type Float%20%28single-precision%29))
  (if (Variables|Default|GetbIsTeleporting)
    (CallFunction|DetectHitPoint)))

(fn StartTeleport
  (Variables|Default|SetbIsTeleporting true)
  (Rendering|SetVisibility (Variables|/Game/BallGame/BP_TeleportTarget.BP_TeleportTarget_C|GetSphere (Variables|Default|GetTeleportTarget)) true false))

(fn StopTeleport
  (bind _hitlocation (Variables|Default|GetHitLocation))
  (Variables|Default|SetbIsTeleporting false)
  (Rendering|SetVisibility (Variables|/Game/BallGame/BP_TeleportTarget.BP_TeleportTarget_C|GetSphere (Variables|Default|GetTeleportTarget)) false false)
  (if (Variables|Default|GetbDetectedHit)
    (Transformation|SetActorLocation (Variables|Default|GetTeleportActor) (Math|Vector|MakeVector (.x _hitlocation) (.y _hitlocation) (+ (.z _hitlocation) (Variables|Default|GetzOffset))) false false)))

(fn DetectHitPoint
  (bind _returnvalue (Transformation|GetWorldLocation))
  (bind (_outhit _returnvalue_2) (Collision|LineTraceByChannel _returnvalue (+ _returnvalue (* (Math|Vector|GetForwardVector) (Variables|Default|GetDistance))) "TraceTypeQuery1" false 0 "None"))
  (Variables|Default|SetHitLocation (.ProjectedLocation (AI|Navigation|ProjectPointtoNavigation (.location _outhit) 0 0 "0, 0, 0")))
  (Variables|Default|SetbDetectedHit _returnvalue_2)
  (Transformation|SetActorLocation (Variables|Default|GetTeleportTarget) (.ProjectedLocation (AI|Navigation|ProjectPointtoNavigation (.location _outhit) 0 0 "0, 0, 0")) false false))

(fn GetZOffset
  (params (self2 :type Actor%20Object%20Reference))
  (bind _returnvalue (Actor|GetComponentbyClass self2 "/Script/Engine.CapsuleComponent"))
  (Utilities|IsValid _returnvalue
    (:Is%20Valid
      (Variables|Default|SetzOffset (Variables|/Script/Engine.CapsuleComponent|GetCapsuleHalfHeight _returnvalue))
      (return))))